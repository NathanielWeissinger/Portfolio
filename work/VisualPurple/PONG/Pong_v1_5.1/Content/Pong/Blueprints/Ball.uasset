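; Pong ball Actor that launches itself at match start, keeps both players' scores and ends the match.
; BeginPlay fires a randomized impulse on the Sphere toward either side along Y.
; Tick watches both Y bounds; crossing one hides the ball, waits on a Delay, recenters it and increments that side's score.
; It then relaunches with a weaker impulse, or shows a game-over widget and pauses when a score reaches 10.
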(event `self.ReceiveBeginPlay`
  ;[1 1 1] Sets score variables, etermine initial direction the ball moves towards at beginning of match
  (set `self.ScoreP1` 0)
  (set `self.ScoreP2` 0)
  (if (`KismetMathLibrary.RandomBool`)
    (`PrimitiveComponent.AddImpulse` (`self.Sphere`) (`KismetMathLibrary.MakeVector` (* (`KismetMathLibrary.RandomFloat`) 1000) (* 1 1200)) "None" true)
    (else
      (`PrimitiveComponent.AddImpulse` (`self.Sphere`) (`KismetMathLibrary.MakeVector` (* (`KismetMathLibrary.RandomFloat`) 1000) (* 1 -1200)) "None" true))))

(event `self.ReceiveTick`
  (params (DeltaSeconds :type "Float (single-precision)"))
  (bind (_returnvalue_x _returnvalue_y) (`KismetMathLibrary.BreakVector` (`self.K2_GetActorLocation`)))
  (bind _returnvalue (+ (`self.ScoreP1`) 1))
  (bind _returnvalue_2 (+ (`self.ScoreP2`) 1))
  ;[1 1 1] Ball Respawn After Scoring, Adds Scores
  (`|ExecutionSequence`
    (:`then_0`
      (if (<= _returnvalue_y -1500.0)
        (set `self.win_side` true)
        (`SceneComponent.SetVisibility` (`self.Sphere`) false false :!label _label)
        (`KismetSystemLibrary.Delay` 1.5)
        (`self.K2_SetActorLocation` (1250.0 1550.0 190.0))
        (`SceneComponent.SetVisibility` (`self.Sphere`) true false)
        (if (`self.win_side`)
          (set `self.ScoreP1` _returnvalue)
          (if (>= _returnvalue 11)
            ;[1 1 1] Activate Game Over screen
            (bind _returnvalue_3 (`|CreateWidget` "/Game/Pong/Blueprints/GameOver.GameOver_C" :!label _label_2))
            (`UserWidget.AddToViewport` _returnvalue_3 0)
            (set `PlayerController.bShowMouseCursor` true (`GameplayStatics.GetPlayerController` 0))
            (`GameplayStatics.SetGamePaused` true)
            (else
              (`PrimitiveComponent.AddImpulse` (`self.Sphere`) (`KismetMathLibrary.MakeVector` (* (`KismetMathLibrary.RandomFloat`) -200) (* 1 -100)) "None" true)))
          (else
            (set `self.ScoreP2` _returnvalue_2)
            (if (>= _returnvalue_2 11)
              (goto _label_2)
              (else
                (`PrimitiveComponent.AddImpulse` (`self.Sphere`) (`KismetMathLibrary.MakeVector` (* (`KismetMathLibrary.RandomFloat`) 200) (* 1 100)) "None" true)))))))
    (:`then_1`
      (if (>= _returnvalue_y 4500.0)
        (set `self.win_side` false)
        (goto _label)))))

(fn `UserConstructionScript`)