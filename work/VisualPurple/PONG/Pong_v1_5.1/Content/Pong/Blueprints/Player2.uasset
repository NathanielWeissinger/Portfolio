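; Player 2 paddle for a Pong game, moved up and down along the X axis by the P2_Up and P2_Down input actions.
; It enables input from player controller 0 on BeginPlay.
; Holding a key sets a flag that drives a short Delay loop, nudging the paddle by a fixed local offset until release or until it reaches that side's hard-coded X limit.
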(event `self.ReceiveBeginPlay`
  ;[1 1 1] Enable Actor Input
  (`self.EnableInput` (`GameplayStatics.GetPlayerController` 0)))

(event `InputAction|P2_Down`
  (params (Key :type "Key Structure"))
  (bind _returnvalue_x (`KismetMathLibrary.BreakVector` (`self.K2_GetActorLocation`)))
  ;[1 1 1] Move Down
  (:`Pressed`
    (set `self.hold_down2` true)
    (if (`self.hold_down2`) :!label _label
      (if (not (>= _returnvalue_x 2000.0))
        (`self.K2_AddActorLocalOffset` (`KismetMathLibrary.MakeVector` (+ 0.0 30.0)))
        (`KismetSystemLibrary.Delay` 0.01)
        (goto _label))))
  (:`Released`
    (set `self.hold_down2` false)
    (goto _label)))

(event `InputAction|P2_Up`
  (params (Key :type "Key Structure"))
  (bind _returnvalue_x (`KismetMathLibrary.BreakVector` (`self.K2_GetActorLocation`)))
  ;[1 1 1] Move Up
  (:`Pressed`
    (set `self.hold_up2` true)
    (if (`self.hold_up2`) :!label _label_2
      (if (not (<= _returnvalue_x 520.0))
        (`self.K2_AddActorLocalOffset` (`KismetMathLibrary.MakeVector` (+ 0.0 -30.0)))
        (`KismetSystemLibrary.Delay` 0.01)
        (goto _label_2))))
  (:`Released`
    (set `self.hold_up2` false)
    (goto _label_2)))

(fn `UserConstructionScript`)