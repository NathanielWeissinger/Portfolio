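; CPU paddle for Pong that tracks the Ball actor along X and also carries Player 2 up/down input handlers.
; A throttled Tick looks up the Ball, caches its sphere's relative location and calls Move, which drives MoveComponentTo on the Cube, stopping at preset boundaries.
; P2 input runs Delay-based loops that nudge the whole actor while held, within position limits.
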(event `self.ReceiveTick`
  (params (DeltaSeconds :type "Float (single-precision)"))
  ;[1 1 1] Move CPU Player
  (bind _returnvalue (`GameplayStatics.GetActorOfClass` "/Game/Pong/Blueprints/Ball.Ball_C"))
  (set `self.ball_location` (`SceneComponent.RelativeLocation` (`/Game/Pong/Blueprints/Ball.Sphere` _returnvalue)))
  (`self.Move`))

(event `self.ReceiveBeginPlay`
  ;[1 1 1] Set Tick Interval
  (bind _output_get (set `self.Tick Interval` 0.2))
  (`self.SetActorTickInterval` _output_get))

(event `Move`
  (bind _ball_location_x (`KismetMathLibrary.BreakVector` (`self.ball_location`)))
  ;[1 1 1] AI For Ball Tracking (stops at prespecified boundaries)
  (`|ExecutionSequence`
    (:`then_0`
      (if (>= _ball_location_x 1780.0)
        (goto _label :!via `Stop`)
        (elif (<= _ball_location_x 220.0)
          (goto _label :!via `Stop`)
          (else
            (`KismetSystemLibrary.MoveComponentTo` (`self.Cube`) (`KismetMathLibrary.MakeVector` (+ _ball_location_x -1000.0)) (struct) false false 0.5 :!label _label)))))))

(event `InputAction|P2_Down`
  (params (Key :type "Key Structure"))
  (bind _returnvalue_x (`KismetMathLibrary.BreakVector` (`self.K2_GetActorLocation`)))
  ;[1 1 1] Move Down
  (:`Pressed`
    (set `self.hold_down2` true)
    (if (`self.hold_down2`) :!label _label_2
      (if (not (>= _returnvalue_x 2000.0))
        (`self.K2_AddActorLocalOffset` (`KismetMathLibrary.MakeVector` (+ 0.0 30.0)))
        (`KismetSystemLibrary.Delay` 0.01)
        (goto _label_2))))
  (:`Released`
    (set `self.hold_down2` false)
    (goto _label_2)))

(event `InputAction|P2_Up`
  (params (Key :type "Key Structure"))
  (bind _returnvalue_x (`KismetMathLibrary.BreakVector` (`self.K2_GetActorLocation`)))
  ;[1 1 1] Move Up
  (:`Pressed`
    (set `self.hold_up2` true)
    (if (`self.hold_up2`) :!label _label_3
      (if (not (<= _returnvalue_x 520.0))
        (`self.K2_AddActorLocalOffset` (`KismetMathLibrary.MakeVector` (+ 0.0 -30.0)))
        (`KismetSystemLibrary.Delay` 0.01)
        (goto _label_3))))
  (:`Released`
    (set `self.hold_up2` false)
    (goto _label_3)))

(fn `UserConstructionScript`)