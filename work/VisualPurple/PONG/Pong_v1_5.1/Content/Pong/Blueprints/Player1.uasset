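; Player 1 paddle for a Pong game, moved along the X axis by the P1_Up and P1_Down input actions.
; Each press sets a hold flag and starts a self-repeating Delay loop that offsets the actor in fixed steps, in place of Tick.
; A loop stops when its key release clears the flag or the paddle reaches that direction's hard-coded X limit.
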(event `InputAction|P1_Down`
  (params (Key :type "Key Structure"))
  (bind _returnvalue_x (`KismetMathLibrary.BreakVector` (`self.K2_GetActorLocation`)))
  ;[1 1 1] Move Down
  (:`Pressed`
    (set `self.hold_down1` true)
    (if (`self.hold_down1`) :!label _label
      (if (not (>= _returnvalue_x 2000.0))
        (`self.K2_AddActorLocalOffset` (`KismetMathLibrary.MakeVector` (+ 0.0 30.0)))
        (`KismetSystemLibrary.Delay` 0.01)
        (goto _label))))
  (:`Released`
    (set `self.hold_down1` false)
    (goto _label)))

(event `InputAction|P1_Up`
  (params (Key :type "Key Structure"))
  (bind _returnvalue_x (`KismetMathLibrary.BreakVector` (`self.K2_GetActorLocation`)))
  ;[1 1 1] Move Up
  (:`Pressed`
    (set `self.hold_up1` true)
    (if (`self.hold_up1`) :!label _label_2
      (if (not (<= _returnvalue_x 520.0))
        (`self.K2_AddActorLocalOffset` (`KismetMathLibrary.MakeVector` (+ 0.0 -30.0)))
        (`KismetSystemLibrary.Delay` 0.01)
        (goto _label_2))))
  (:`Released`
    (set `self.hold_up1` false)
    (goto _label_2)))

(fn `UserConstructionScript`)