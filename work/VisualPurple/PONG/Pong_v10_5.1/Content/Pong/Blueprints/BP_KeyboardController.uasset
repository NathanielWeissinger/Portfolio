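; Keyboard controller for two-player local Pong that drives both player pawns from shared input.
; On BeginPlay it caches the two BP_PlayerPawns, then Enhanced Input up and down actions call press and release functions on the matching pawn.
; A dev menu action lazily creates WBP_DevMenu, shows it with mouse cursor and UI-only input, and pauses the game.
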(event `EnhancedInput|/Game/Pong/Input/Actions/IA_P1_MoveUp`
  (params (ActionValue :type Boolean) (ElapsedSeconds :type "Float (double-precision)") (TriggeredSeconds :type "Float (double-precision)") (InputAction :type "InputAction Object Reference" :default "/Game/Pong/Input/Actions/IA_P1_MoveUp.IA_P1_MoveUp"))
  ;[1 1 1] P1 Move Up
  (:`Triggered`
    (`/Game/Pong/Blueprints/BP_PlayerPawn.Press_MoveUp` (`self.player1_pawn`)))
  (:`Completed`
    (`/Game/Pong/Blueprints/BP_PlayerPawn.Release_MoveUp` (`self.player1_pawn`))))

(event `self.ReceiveBeginPlay`
  ;[1 1 1] Initialize Player Pawns
  (bind _asbp_player_pawn (cast `/Game/Pong/Blueprints/BP_PlayerPawn` (`GameplayStatics.GetPlayerPawn` 0)))
  (set `self.player1_pawn` _asbp_player_pawn)
  (bind _asbp_player_pawn_2 (cast `/Game/Pong/Blueprints/BP_PlayerPawn` (`GameplayStatics.GetPlayerPawn` 1)))
  (set `self.player2_pawn` _asbp_player_pawn_2))

(event `EnhancedInput|/Game/Pong/Input/Actions/IA_P1_MoveDown`
  (params (ActionValue :type Boolean) (ElapsedSeconds :type "Float (double-precision)") (TriggeredSeconds :type "Float (double-precision)") (InputAction :type "InputAction Object Reference" :default "/Game/Pong/Input/Actions/IA_P1_MoveDown.IA_P1_MoveDown"))
  ;[1 1 1] P1 Move Down
  (:`Triggered`
    (`/Game/Pong/Blueprints/BP_PlayerPawn.Press_MoveDown` (`self.player1_pawn`)))
  (:`Completed`
    (`/Game/Pong/Blueprints/BP_PlayerPawn.Release_MoveDown` (`self.player1_pawn`))))

(event `EnhancedInput|/Game/Pong/Input/Actions/IA_DevMenuPullup`
  (params (ActionValue :type Boolean) (ElapsedSeconds :type "Float (double-precision)") (TriggeredSeconds :type "Float (double-precision)") (InputAction :type "InputAction Object Reference" :default "/Game/Pong/Input/Actions/IA_DevMenuPullup.IA_DevMenuPullup"))
  ;[1 1 1] Developer Menu (Press Tab]
  (:`Started`
    (`self.StartDevMenu`)))

(event `EnhancedInput|/Game/Pong/Input/Actions/IA_P2_MoveUp`
  (params (ActionValue :type Boolean) (ElapsedSeconds :type "Float (double-precision)") (TriggeredSeconds :type "Float (double-precision)") (InputAction :type "InputAction Object Reference" :default "/Game/Pong/Input/Actions/IA_P2_MoveUp.IA_P2_MoveUp"))
  ;[1 1 1] P2 Move Up
  (:`Triggered`
    (`/Game/Pong/Blueprints/BP_PlayerPawn.Press_MoveUp` (`self.player2_pawn`)))
  (:`Completed`
    (`/Game/Pong/Blueprints/BP_PlayerPawn.Release_MoveUp` (`self.player2_pawn`))))

(event `EnhancedInput|/Game/Pong/Input/Actions/IA_P2_MoveDown`
  (params (ActionValue :type Boolean) (ElapsedSeconds :type "Float (double-precision)") (TriggeredSeconds :type "Float (double-precision)") (InputAction :type "InputAction Object Reference" :default "/Game/Pong/Input/Actions/IA_P2_MoveDown.IA_P2_MoveDown"))
  ;[1 1 1] P2 Move Down
  (:`Triggered`
    (`/Game/Pong/Blueprints/BP_PlayerPawn.Press_MoveDown` (`self.player2_pawn`)))
  (:`Completed`
    (`/Game/Pong/Blueprints/BP_PlayerPawn.Release_MoveDown` (`self.player2_pawn`))))

(fn `StartDevMenu`
  (bind _returnvalue (`GameplayStatics.GetPlayerController` 0))
  (bind _devmenu_widget (`self.devmenu_widget`))
  ;[1 1 1] Starts the Developer Menu Widget
  (`/Engine/EditorBlueprintResources/StandardMacros.IsValid` _devmenu_widget
    (:`Is Valid`
      _)
    (:`Is Not Valid`
      (bind _returnvalue_2 (`|CreateWidget` "/Game/Pong/UI/WBP_DevMenu.WBP_DevMenu_C"))
      (set `self.devmenu_widget` _returnvalue_2)))
  ;;[1 1 1] Enables Mouse/Keyboard Presses
  (set `PlayerController.bShowMouseCursor` true _returnvalue)
  (`WidgetBlueprintLibrary.SetInputMode_UIOnlyEx` _returnvalue _devmenu_widget)
  (`UserWidget.AddToViewport` _devmenu_widget 0)
  (`GameplayStatics.SetGamePaused` true)
  (`Widget.SetKeyboardFocus` _devmenu_widget))

(fn `UserConstructionScript`)