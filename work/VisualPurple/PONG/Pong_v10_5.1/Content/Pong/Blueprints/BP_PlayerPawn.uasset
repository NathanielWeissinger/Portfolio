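; Player paddle pawn for Pong that moves on keyboard input and deflects the ball.
; Move presses apply a physics impulse to the Cube and releases apply the opposite one.
; On a ball hit it waits two ticks, sets an angle-adjusted velocity from the relative hit point, then calls the ball's hit impulse.
; Its own hit-ratio and angle math functions are not called from the event graph.
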(event `self.ReceiveBeginPlay`
  ;[1 1 1] Set Ball Actor reference for future use
  (bind _returnvalue (`GameplayStatics.GetActorOfClass` "/Game/Pong/Blueprints/BP_BallPawn.BP_BallPawn_C"))
  (set `self.ball_actor` _returnvalue)
  (bind _asplayer_controller (cast `PlayerController` (`GameplayStatics.GetPlayerController` 0)))
  (bind _returnvalue_2 (pcsubsystem `EnhancedInputLocalPlayerSubsystem` _asplayer_controller))
  (`/Engine/EditorBlueprintResources/StandardMacros.IsValid` _returnvalue_2
    (:`Is Valid`
      (`EnhancedInputSubsystemInterface.AddMappingContext` _returnvalue_2 "/Game/Pong/Input/IMC_Keyboard.IMC_Keyboard" 0 (struct)))))

(event `Press_MoveUp`
  ;[1 1 1] Move Up
  (`PrimitiveComponent.AddImpulse` (`self.Cube`) (100000.0 0.0 0.0) "None" false))

(event `Release_MoveUp`
  ;[1 1 1] Move Up
  (`PrimitiveComponent.AddImpulse` (`self.Cube`) (-100000.0 0.0 0.0) "None" false))

(event `Press_MoveDown`
  ;[1 1 1] Move Down
  (`PrimitiveComponent.AddImpulse` (`self.Cube`) (-100000.0 0.0 0.0) "None" false))

(event `Release_MoveDown`
  ;[1 1 1] Move Down
  (`PrimitiveComponent.AddImpulse` (`self.Cube`) (100000.0 0.0 0.0) "None" false))

(event `self.ReceiveHit`
  (params (MyComp :type "PrimitiveComponent Object Reference") (Other :type "Actor Object Reference") (OtherComp :type "PrimitiveComponent Object Reference") (bSelfMoved :type Boolean) (HitLocation :type "Vector Structure") (HitNormal :type "Vector Structure") (NormalImpulse :type "Vector Structure") (Hit :type "HitResult Structure (by ref)"))
  (bind _asbp_ball_pawn (cast `/Game/Pong/Blueprints/BP_BallPawn` Other :!pure true))
  (bind _cube (`self.Cube`))
  ;[1 1 1] Upon Hit, Add Impulse to Ball
  ;;[1 1 1] If hit by ball, get location of hit
  (if (== Other (`self.ball_actor`))
    (bind _relativehitlocation (`Cpp_AdvancedFunctionLibrary.GetRelativeHitLocation` HitLocation (`SceneComponent.K2_GetComponentLocation` _cube)))
    ;;[1 1 1] Hit to Length Ratio: 1 (top) to -1 (bottom) of paddle
    (`KismetSystemLibrary.DelayUntilNextTick`)
    (`KismetSystemLibrary.DelayUntilNextTick`)
    (bind _newtargetvector (`Cpp_AdvancedFunctionLibrary.SetHitDegreeChangeXY` _asbp_ball_pawn _cube HitNormal _relativehitlocation 40.0))
    (`PrimitiveComponent.SetAllPhysicsLinearVelocity` (`/Game/Pong/Blueprints/BP_BallPawn.Sphere` _asbp_ball_pawn) (`KismetMathLibrary.MakeVector` (.x _newtargetvector) (.y _newtargetvector)) false)
    (`/Game/Pong/Blueprints/BP_BallPawn.AddBallImpulseOnHit` _asbp_ball_pawn)))

(fn `GetLengthHitRatio`
  (params (RelativeX :type "Float (double-precision)") (RelativeY :type "Float (double-precision)") (RelativeZ :type "Float (double-precision)"))
  (returns (LengthHitRatio :type "Float (double-precision)"))
  (locals (LHR :type "Float (double-precision)"))
  (bind (_origin _boxextent) (`KismetSystemLibrary.GetComponentBounds` (`self.Cube`)))
  (bind _returnvalue (/ (`KismetMathLibrary.Sqrt` (- (`KismetMathLibrary.VSizeSquared` (`KismetMathLibrary.MakeVector` RelativeX RelativeY RelativeZ)) (`KismetMathLibrary.Square` (.y _boxextent)))) (.x _boxextent)))
  (if (<= RelativeX 0.0)
    (set `local.LHR` _returnvalue)
    (else
      (set `local.LHR` (* -1.0 _returnvalue))))
  (return (`local.LHR`)))

(fn `GetRelativeLocation`
  (params (hitlocation :type "Vector Structure") (origin :type "Vector Structure"))
  (returns (locallocation :type "Vector Structure"))
  (return (- hitlocation origin)))

(fn `UserConstructionScript`)