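; Game instance for Pong that holds the match options, such as ball speed, gravity, shape presets, max score and camera scrolling, and persists them.
; On Init it loads the OptionsSave slot and copies its values into its own variables.
; If that load or cast fails, it creates a Pong_SaveGame from its current values.
; Either way, it then writes the save back to the slot.
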(event `self.ReceiveInit`
  (bind _returnvalue (`GameplayStatics.LoadGameFromSlot` "OptionsSave"))
  (bind _aspong_save_game (cast `/Game/Pong/Blueprints/Pong_SaveGame` _returnvalue)
    (:`then`
      ;[1 1 1] <-- Load
      (set `self.OptionsSave` _aspong_save_game)
      (`self.LoadVariablesFromSave`))
    (:`CastFailed`
      ;[1 1 1] Save -->
      (bind _returnvalue_2 (`GameplayStatics.CreateSaveGameObject` "/Game/Pong/Blueprints/Pong_SaveGame.Pong_SaveGame_C"))
      (set `self.OptionsSave` _returnvalue_2)
      (`self.SaveVariablesFromInstance`)))
  (`GameplayStatics.SaveGameToSlot` (`self.OptionsSave`) "OptionsSave"))

(fn `LoadVariablesFromSave`
  (bind _optionssave (`self.OptionsSave`))
  (set `self.BallSpeed` (`/Game/Pong/Blueprints/Pong_SaveGame.BallSpeed` _optionssave))
  (set `self.BallIncrement` (`/Game/Pong/Blueprints/Pong_SaveGame.BallIncrement` _optionssave))
  (set `self.bEnableGravity` (`/Game/Pong/Blueprints/Pong_SaveGame.EnableGravity` _optionssave))
  (set `self.bGravityUp` (`/Game/Pong/Blueprints/Pong_SaveGame.bGravityUp` _optionssave))
  (set `self.bGravityDown` (`/Game/Pong/Blueprints/Pong_SaveGame.bGravityDown` _optionssave))
  (set `self.bGravityChaotic` (`/Game/Pong/Blueprints/Pong_SaveGame.bGravityChaotic` _optionssave))
  (set `self.GravityPresets` (`/Game/Pong/Blueprints/Pong_SaveGame.GravityPresets` _optionssave))
  (set `self.MaxScore` (`/Game/Pong/Blueprints/Pong_SaveGame.MaxScore` _optionssave))
  (set `self.ShapePresets` (`/Game/Pong/Blueprints/Pong_SaveGame.ShapePresets` _optionssave))
  (set `self.bSpeedUp` (`/Game/Pong/Blueprints/Pong_SaveGame.bSpeedUp` _optionssave))
  (set `self.bCameraScrolling` (`/Game/Pong/Blueprints/Pong_SaveGame.bCameraScrolling` _optionssave))
  (set `self.CameraSpeed` (`/Game/Pong/Blueprints/Pong_SaveGame.CameraSpeed` _optionssave)))

(fn `SaveVariablesFromInstance`
  (bind _optionssave (`self.OptionsSave`))
  (set `/Game/Pong/Blueprints/Pong_SaveGame.BallSpeed` (`self.BallSpeed`) _optionssave)
  (set `/Game/Pong/Blueprints/Pong_SaveGame.BallIncrement` (`self.BallIncrement`) _optionssave)
  (set `/Game/Pong/Blueprints/Pong_SaveGame.EnableGravity` (`self.bEnableGravity`) _optionssave)
  (set `/Game/Pong/Blueprints/Pong_SaveGame.bGravityUp` (`self.bGravityUp`) _optionssave)
  (set `/Game/Pong/Blueprints/Pong_SaveGame.bGravityDown` (`self.bGravityDown`) _optionssave)
  (set `/Game/Pong/Blueprints/Pong_SaveGame.bGravityChaotic` (`self.bGravityChaotic`) _optionssave)
  (set `/Game/Pong/Blueprints/Pong_SaveGame.GravityPresets` (`self.GravityPresets`) _optionssave)
  (set `/Game/Pong/Blueprints/Pong_SaveGame.MaxScore` (`self.MaxScore`) _optionssave)
  (set `/Game/Pong/Blueprints/Pong_SaveGame.ShapePresets` (`self.ShapePresets`) _optionssave)
  (set `/Game/Pong/Blueprints/Pong_SaveGame.bSpeedUp` (`self.bSpeedUp`) _optionssave)
  (set `/Game/Pong/Blueprints/Pong_SaveGame.bCameraScrolling` (`self.bCameraScrolling`) _optionssave)
  (set `/Game/Pong/Blueprints/Pong_SaveGame.CameraSpeed` (`self.CameraSpeed`) _optionssave))