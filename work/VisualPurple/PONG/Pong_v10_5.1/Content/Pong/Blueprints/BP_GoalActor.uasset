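; Goal actor for a Pong game that awards a point when something overlaps it while the ball is not flagged as Reset.
; On BeginPlay it caches the Pong game state and finds the BP_BallPawn to read that flag.
; The GetGoalNumber macro branches on GoalPlayerNumber to credit the opposing player, then the game state tracks the score.
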(event `self.ReceiveBeginPlay`
  ;[1 1 1] Set GameState object for score reference
  (bind _aspong_game_state_base (cast `/Game/Pong/Blueprints/Pong_GameStateBase` (`GameplayStatics.GetGameState`)))
  (set `self.gamestate` _aspong_game_state_base)
  (bind _returnvalue (`GameplayStatics.GetActorOfClass` "/Game/Pong/Blueprints/BP_BallPawn.BP_BallPawn_C"))
  (set `self.ball_actor` _returnvalue))

(event `self.ReceiveActorBeginOverlap`
  (params (OtherActor :type "Actor Object Reference"))
  (bind _gamestate (`self.gamestate`))
  ;[1 1 1] When Ball overlaps Goal, add and track score NOTE: goal number needs to eventually depend on WHO scored the goal, rather than which goal side the ball touched
  (if (not (`/Game/Pong/Blueprints/BP_BallPawn.bReset` (`self.ball_actor`)))
    (`self.GetGoalNumber`
      (:`then`
        (`/Game/Pong/Blueprints/Pong_GameStateBase.AddScoreP2` _gamestate))
      (:`then2`
        (`/Game/Pong/Blueprints/Pong_GameStateBase.AddScoreP1` _gamestate)))
    (`/Game/Pong/Blueprints/Pong_GameStateBase.TrackScore` _gamestate)))

(fn `UserConstructionScript`)