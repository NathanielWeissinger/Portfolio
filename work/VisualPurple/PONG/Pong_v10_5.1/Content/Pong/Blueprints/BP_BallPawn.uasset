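; Physics-driven ball pawn for Pong, configured from Pong_GameInstance with speed, gravity and shape options, and launched randomly at match start.
; Tick adds optional up, down or chaotic X-axis velocity using Pluto, Earth or Jupiter gravity presets.
; Sphere drives all movement, while shape selection toggles visibility and collision across sphere, cube, cone and L-shape meshes.
; Functions handle goal resets, side-based relaunches and speed increases; ChangeBallDirectionOnHit is empty.
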(event `self.ReceiveBeginPlay`
  (bind _ballspeed (`self.BallSpeed`))
  (bind _ballspeed_2 (`self.BallSpeed`))
  ;[1 1 1] Sets score variables, determine initial direction the ball moves towards at beginning of match
  (`self.LoadVariables`)
  (if (`KismetMathLibrary.RandomBool`)
    (`PrimitiveComponent.AddImpulse` (`self.Sphere`) (`KismetMathLibrary.MakeVector` (* (`KismetMathLibrary.RandomFloatInRange` -1.0 1.0) _ballspeed) (* 1 _ballspeed)) "None" true)
    (else
      (`PrimitiveComponent.AddImpulse` (`self.Sphere`) (`KismetMathLibrary.MakeVector` (* (`KismetMathLibrary.RandomFloatInRange` -1.0 1.0) _ballspeed_2) (* -1 _ballspeed_2)) "None" true))))

(event `self.ReceiveTick`
  (params (DeltaSeconds :type "Float (single-precision)"))
  ;[1 1 1] Event Tick Gravity
  (if (`self.bReset`)
    _
    (elif (`self.bEnableGravity`)
      (if (`self.bGravityChaotic`)
        (`self.SetGravity` (`KismetMathLibrary.RandomFloatInRange` -1.0 1.0) (`self.gravity_variable`))
        (elif (`self.bGravityUp`)
          (`self.SetGravity` -1.0 (`self.gravity_variable`))
          (elif (`self.bGravityDown`)
            (`self.SetGravity` 1.0 (`self.gravity_variable`))))))))

(event `ChangeShape`
  (bind _ball_shape (`self.ball_shape`))
  ;[1 1 1] Changes the shape of the ball and enables collisions
  (`self.SetVisibility` _ball_shape true)
  (`self.SetCollision` _ball_shape))

(fn `AddBallImpulseOnHit`
  (bind (_returnvalue_x _returnvalue_y) (`KismetMathLibrary.BreakVector` (`self.GetVelocity`)))
  (bind _ball_increment (`self.ball_increment`))
  (bind _sphere (`self.Sphere`))
  (bind _returnvalue (* _returnvalue_y (+ (* _ball_increment 0.001) 1.0)))
  (bind _returnvalue_2 (* _returnvalue_x (+ (* _ball_increment 0.001) 1.0)))
  ;[1 1 1] Adds Impulse each time it collides with a Player/CPU
  (if (`self.bSpeedUp`)
    (if (`self.bEnableGravity`)
      (`PrimitiveComponent.SetAllPhysicsLinearVelocity` _sphere (`KismetMathLibrary.MakeVector` (+ _returnvalue_2 -500.0) _returnvalue) false)
      (else
        (`PrimitiveComponent.SetAllPhysicsLinearVelocity` _sphere (`KismetMathLibrary.MakeVector` _returnvalue_2 _returnvalue) false)))))

(fn `ChangeBallDirectionOnHit`
  ;[1 1 1] add impulse depending on ratio of magnitude, use cosine and sine to split x and y impulses, set negative to y impulse to decrease speed
)

(fn `IncreaseBallVelocity`
  ;[1 1 1] Increases Ball Velocity After Reset
  (set `self.BallSpeed` (+ (`self.BallSpeed`) (`self.ball_increment`))))

(fn `LoadVariables`
  (bind _aspong_game_instance (cast `/Game/Pong/Blueprints/Pong_GameInstance` (`GameplayStatics.GetGameInstance`)))
  (set `self.BallSpeed` (`/Game/Pong/Blueprints/Pong_GameInstance.BallSpeed` _aspong_game_instance))
  (set `self.ball_increment` (`/Game/Pong/Blueprints/Pong_GameInstance.BallIncrement` _aspong_game_instance))
  (set `self.bEnableGravity` (`/Game/Pong/Blueprints/Pong_GameInstance.bEnableGravity` _aspong_game_instance))
  (set `self.bGravityChaotic` (`/Game/Pong/Blueprints/Pong_GameInstance.bGravityChaotic` _aspong_game_instance))
  (set `self.bGravityUp` (`/Game/Pong/Blueprints/Pong_GameInstance.bGravityUp` _aspong_game_instance))
  (set `self.bGravityDown` (`/Game/Pong/Blueprints/Pong_GameInstance.bGravityDown` _aspong_game_instance))
  (bind _output_get (set `self.gravity_presets` (`/Game/Pong/Blueprints/Pong_GameInstance.GravityPresets` _aspong_game_instance)))
  (if (== _output_get 0)
    (set `self.gravity_variable` (`self.PlutoGravity`))
    (set `self.ball_shape` (`/Game/Pong/Blueprints/Pong_GameInstance.ShapePresets` _aspong_game_instance) :!label _label)
    (`self.ChangeShape`)
    (set `self.bSpeedUp` (`/Game/Pong/Blueprints/Pong_GameInstance.bSpeedUp` _aspong_game_instance))
    (elif (== _output_get 1)
      (set `self.gravity_variable` (`self.EarthGravity`))
      (goto _label)
      (elif (== _output_get 2)
        (set `self.gravity_variable` (`self.JupiterGravity`))
        (goto _label)))))

(fn `ResetBallLocation`
  (bind _sphere (`self.Sphere`))
  ;[1 1 1] Resets Ball Location After Goal Is Scored
  (`SceneComponent.SetVisibility` _sphere false false)
  (`self.K2_SetActorLocation` (1250.0 1550.0 190.0))
  (`PrimitiveComponent.SetAllPhysicsLinearVelocity` _sphere (0.0 0.0 0.0) false)
  (`PrimitiveComponent.SetAllPhysicsAngularVelocityInDegrees` _sphere (0.0 0.0 0.0) false)
  (`self.K2_SetActorRotation` (struct)))

(fn `ResetBallVelocity`
  (bind _sphere (`self.Sphere`))
  (bind _ballspeed (`self.BallSpeed`))
  ;[1 1 1] Sets New Ball Velocity After Reset
  (`self.SetVisibility` (`self.ball_shape`) true)
  (if (`self.bWinSide`)
    (`PrimitiveComponent.AddImpulse` _sphere (`KismetMathLibrary.MakeVector` (* (`KismetMathLibrary.RandomFloatInRange` -1.0 1.0) _ballspeed) (`KismetMathLibrary.FClamp` (* (`KismetMathLibrary.RandomFloatInRange` 1.0 2.0) _ballspeed) 1200.0 5000.0)) "None" true)
    (else
      (`PrimitiveComponent.AddImpulse` _sphere (`KismetMathLibrary.MakeVector` (* (`KismetMathLibrary.RandomFloatInRange` -1.0 1.0) _ballspeed) (`KismetMathLibrary.FClamp` (* (`KismetMathLibrary.RandomFloatInRange` 1.0 2.0) _ballspeed -1.0) -5000.0 -1200.0)) "None" true))))

(fn `SetCollision`
  (params (ball_shape :type Integer))
  (if (== ball_shape 0)
    (`PrimitiveComponent.SetCollisionEnabled` (`self.Sphere`) "QueryAndPhysics")
    (`PrimitiveComponent.SetCollisionEnabled` (`self.Cube`) "NoCollision")
    (`PrimitiveComponent.SetCollisionEnabled` (`self.L Shape`) "NoCollision")
    (`PrimitiveComponent.SetCollisionEnabled` (`self.L2`) "NoCollision")
    (`PrimitiveComponent.SetCollisionEnabled` (`self.Cone`) "NoCollision")
    (elif (== ball_shape 1)
      (`PrimitiveComponent.SetCollisionEnabled` (`self.Cube`) "QueryAndPhysics")
      (`PrimitiveComponent.SetCollisionEnabled` (`self.L Shape`) "NoCollision")
      (`PrimitiveComponent.SetCollisionEnabled` (`self.L2`) "NoCollision")
      (`PrimitiveComponent.SetCollisionEnabled` (`self.Cone`) "NoCollision")
      (elif (== ball_shape 2)
        (`PrimitiveComponent.SetCollisionEnabled` (`self.Cone`) "QueryAndPhysics")
        (`PrimitiveComponent.SetCollisionEnabled` (`self.Cube`) "NoCollision")
        (`PrimitiveComponent.SetCollisionEnabled` (`self.L Shape`) "NoCollision")
        (`PrimitiveComponent.SetCollisionEnabled` (`self.L2`) "NoCollision")
        (elif (== ball_shape 3)
          (`PrimitiveComponent.SetCollisionEnabled` (`self.L Shape`) "QueryAndPhysics")
          (`PrimitiveComponent.SetCollisionEnabled` (`self.L2`) "QueryAndPhysics")
          (`PrimitiveComponent.SetCollisionEnabled` (`self.Cube`) "NoCollision")
          (`PrimitiveComponent.SetCollisionEnabled` (`self.Cone`) "NoCollision"))))))

(fn `SetGravity`
  (params (direction :type "Float (double-precision)") (gravity :type "Float (double-precision)"))
  (`PrimitiveComponent.SetPhysicsLinearVelocity` (`self.Sphere`) (`KismetMathLibrary.MakeVector` (* gravity direction)) true "None"))

(fn `SetVisibility`
  (params (ballshape :type Integer) (visibility :type Boolean))
  (if (== ballshape 0)
    (`SceneComponent.SetVisibility` (`self.Sphere`) visibility false)
    (`SceneComponent.SetVisibility` (`self.Cube`) (not visibility) false)
    (`SceneComponent.SetVisibility` (`self.L Shape`) (not visibility) false)
    (`SceneComponent.SetVisibility` (`self.L2`) (not visibility) false)
    (`SceneComponent.SetVisibility` (`self.Cone`) (not visibility) false)
    (elif (== ballshape 1)
      (`SceneComponent.SetVisibility` (`self.Cube`) visibility false)
      (`SceneComponent.SetVisibility` (`self.L Shape`) (not visibility) false)
      (`SceneComponent.SetVisibility` (`self.L2`) (not visibility) false)
      (`SceneComponent.SetVisibility` (`self.Sphere`) (not visibility) false)
      (`SceneComponent.SetVisibility` (`self.Cone`) (not visibility) false)
      (elif (== ballshape 2)
        (`SceneComponent.SetVisibility` (`self.Cone`) visibility false)
        (`SceneComponent.SetVisibility` (`self.Cube`) (not visibility) false)
        (`SceneComponent.SetVisibility` (`self.L Shape`) (not visibility) false)
        (`SceneComponent.SetVisibility` (`self.L2`) (not visibility) false)
        (`SceneComponent.SetVisibility` (`self.Sphere`) (not visibility) false)
        (elif (== ballshape 3)
          (`SceneComponent.SetVisibility` (`self.L Shape`) visibility false)
          (`SceneComponent.SetVisibility` (`self.L2`) visibility false)
          (`SceneComponent.SetVisibility` (`self.Cube`) (not visibility) false)
          (`SceneComponent.SetVisibility` (`self.Sphere`) (not visibility) false)
          (`SceneComponent.SetVisibility` (`self.Cone`) (not visibility) false))))))

(fn `UserConstructionScript`)