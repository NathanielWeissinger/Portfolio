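; CPU-controlled Pong paddle that tracks the ball and steers its rebound on contact.
; A throttled Tick reads the ball's location and runs Move, which slides the Cube along X with MoveComponentTo, stopping at preset boundaries.
; On a ball hit, the offset from paddle center becomes a signed length ratio that skews the reflected angle while keeping speed.
; The new velocity is applied except at the paddle's extreme ends, then the ball adds its impulse.
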(event `self.ReceiveBeginPlay`
  ;[1 1 1] Set Tick Interval and Gets Ball Actor
  (bind _output_get (set `self.Tick Interval` 0.2))
  (`self.SetActorTickInterval` _output_get)
  (bind _returnvalue (`GameplayStatics.GetActorOfClass` "/Game/Pong/Blueprints/BP_BallPawn.BP_BallPawn_C"))
  (set `self.ball_actor` _returnvalue))

(event `self.ReceiveTick`
  (params (DeltaSeconds :type "Float (single-precision)"))
  ;[1 1 1] Move CPU Player
  (set `self.ball_location` (`SceneComponent.RelativeLocation` (`/Game/Pong/Blueprints/BP_BallPawn.Sphere` (`self.ball_actor`))))
  (`self.Move`))

(event `Move`
  (bind _ball_location_x (`KismetMathLibrary.BreakVector` (`self.ball_location`)))
  (bind _returnvalue_x (`KismetMathLibrary.BreakVector` (`SceneComponent.K2_GetComponentLocation` (`self.Cube`))))
  ;[1 1 1] AI For Ball Tracking (stops at prespecified boundaries)
  (`|ExecutionSequence`
    (:`then_0`
      (if (and (or (>= _returnvalue_x 1860.0) (<= _returnvalue_x 550.0)) (or (>= _ball_location_x 2090.0) (<= _ball_location_x 400.0)))
        (goto _label :!via `Stop`)
        (else
          (`KismetSystemLibrary.MoveComponentTo` (`self.Cube`) (`KismetMathLibrary.MakeVector` (+ _ball_location_x -1200.0)) (struct) false false 0.5 :!label _label))))))

(event `self.ReceiveHit`
  (params (MyComp :type "PrimitiveComponent Object Reference") (Other :type "Actor Object Reference") (OtherComp :type "PrimitiveComponent Object Reference") (bSelfMoved :type Boolean) (HitLocation :type "Vector Structure") (HitNormal :type "Vector Structure") (NormalImpulse :type "Vector Structure") (Hit :type "HitResult Structure (by ref)"))
  (bind _asbp_ball_pawn (cast `/Game/Pong/Blueprints/BP_BallPawn` Other :!pure true))
  ;[1 1 1] Upon Hit from Ball, Add Impulse to Ball
  ;;[1 1 1] If hit by ball, get location of hit
  (if (== Other (`self.ball_actor`))
    (bind _locallocation (`self.GetRelativeLocation` HitLocation (`SceneComponent.K2_GetComponentLocation` (`self.Cube`))))
    ;;[1 1 1] Hit to Length Ratio: 1 (top) to -1 (bottom) of paddle
    (bind _lengthhitratio (`self.GetLengthHitRatio` (.x _locallocation) (.y _locallocation) (.z _locallocation)))
    (if (and (>= _lengthhitratio -0.95) (<= _lengthhitratio 0.95))
      (set `self.LengthHitRatio` _lengthhitratio)
      (bind (_newvectorx _newvectory) (`self.SetMaxDegreeChange` _asbp_ball_pawn HitNormal 40.0))
      (`PrimitiveComponent.SetAllPhysicsLinearVelocity` (`/Game/Pong/Blueprints/BP_BallPawn.Sphere` (`self.ball_actor`)) (`KismetMathLibrary.MakeVector` _newvectorx _newvectory) false))
    (`/Game/Pong/Blueprints/BP_BallPawn.AddBallImpulseOnHit` _asbp_ball_pawn)))

(fn `GetLengthHitRatio`
  (params (RelativeX :type "Float (double-precision)") (RelativeY :type "Float (double-precision)") (RelativeZ :type "Float (double-precision)"))
  (returns (LengthHitRatio :type "Float (double-precision)"))
  (locals (LHR :type "Float (double-precision)"))
  (bind (_origin _boxextent) (`KismetSystemLibrary.GetComponentBounds` (`self.Cube`)))
  (bind _returnvalue (/ (`KismetMathLibrary.Sqrt` (- (`KismetMathLibrary.VSizeSquared` (`KismetMathLibrary.MakeVector` RelativeX RelativeY RelativeZ)) (`KismetMathLibrary.Square` (.y _boxextent)))) (.x _boxextent)))
  (if (<= RelativeX 0.0)
    (set `local.LHR` _returnvalue)
    (else
      (set `local.LHR` (* -1.0 _returnvalue))))
  (return (`local.LHR`)))

(fn `GetRelativeLocation`
  (params (hitlocation :type "Vector Structure") (origin :type "Vector Structure"))
  (returns (locallocation :type "Vector Structure"))
  (return (- hitlocation origin)))

(fn `UserConstructionScript`)