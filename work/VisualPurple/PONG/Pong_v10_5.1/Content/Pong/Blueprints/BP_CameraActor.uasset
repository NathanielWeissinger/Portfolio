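; Camera actor for the Pong game that either follows the ball or holds a fixed overhead position.
; On BeginPlay it reads the scrolling flag and camera speed from Pong_GameInstance and caches the BP_BallPawn reference and position.
; Each tick in scrolling mode it offsets itself by the ball's X/Y movement since last frame, scaled by camera speed.
; Otherwise it snaps to a hardcoded location every tick.
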(event `self.ReceiveBeginPlay`
  ;[1 1 1] Initialize Variables
  (`self.LoadVariables`)
  (bind _returnvalue (`GameplayStatics.GetActorOfClass` "/Game/Pong/Blueprints/BP_BallPawn.BP_BallPawn_C"))
  (set `self.ball_actor` _returnvalue)
  (bind (_returnvalue_x _returnvalue_y) (`KismetMathLibrary.BreakVector` (`self.K2_GetActorLocation` _returnvalue)))
  (set `self.prevBallLocX` _returnvalue_x)
  (set `self.prevBallLocY` _returnvalue_y))

(event `self.ReceiveTick`
  (params (DeltaSeconds :type "Float (single-precision)"))
  (bind _cameraspeed (`self.CameraSpeed`))
  (bind (_returnvalue_x _returnvalue_y) (`KismetMathLibrary.BreakVector` (`self.K2_GetActorLocation` (`self.ball_actor`))))
  ;[1 1 1] Track Ball
  (if (`self.bScrolling`)
    (`self.K2_AddActorLocalOffset` (`KismetMathLibrary.MakeVector` (* (- _returnvalue_x (`self.prevBallLocX`)) _cameraspeed) (* (- _returnvalue_y (`self.prevBallLocY`)) _cameraspeed)))
    (`|ExecutionSequence`
      (:`then_0`
        (set `self.prevBallLocX` _returnvalue_x))
      (:`then_1`
        (set `self.prevBallLocY` _returnvalue_y)))
    (else
      (`self.K2_SetActorLocation` (1250.0 1550.0 3050.0)))))

(fn `LoadVariables`
  (bind _aspong_game_instance (cast `/Game/Pong/Blueprints/Pong_GameInstance` (`GameplayStatics.GetGameInstance`)))
  (set `self.bScrolling` (`/Game/Pong/Blueprints/Pong_GameInstance.bCameraScrolling` _aspong_game_instance))
  (set `self.CameraSpeed` (`/Game/Pong/Blueprints/Pong_GameInstance.CameraSpeed` _aspong_game_instance)))

(fn `UserConstructionScript`)