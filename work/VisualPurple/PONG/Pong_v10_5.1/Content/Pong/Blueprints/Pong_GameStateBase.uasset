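; Game state for Pong that runs match setup, scoring and game over.
; Outside the main menu, BeginPlay creates a local player and pawn at each PlayerStart with keyboard input, sets the shared camera, caches the ball and adds the scoreboard.
; Score functions record the point and winning side on the ball.
; TrackScore compares scores to the GameInstance's MaxScore, then either resets the ball or shows a paused game-over screen.
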(event `self.ReceiveBeginPlay`
  (bind _returnvalue (`GameplayStatics.GetPlayerController` 0))
  (bind _returnvalue_2 (`GameplayStatics.GetCurrentLevelName` true))
  (if (not (`KismetStringLibrary.EqualEqual_StrStr` _returnvalue_2 "Main_Menu_Level"))
    (`|ExecutionSequence`
      (:`then_0`
        ;[1 1 1] Spawn Players
        (bind _outactors (`GameplayStatics.GetAllActorsOfClass` "/Script/Engine.PlayerStart"))
        (for (_ _array_index) _outactors
          (`GameplayStatics.CreatePlayer` _array_index)
          (bind _returnvalue_3 (`|SpawnActorFromClass` "/Game/Pong/Blueprints/BP_PlayerPawn.BP_PlayerPawn_C" (`self.GetTransform` (`|GetArrayItem` _outactors _array_index)) "Undefined" "OverrideRootScale" null null))
          (bind _returnvalue_4 (`GameplayStatics.GetPlayerController` _array_index))
          (`Controller.Possess` _returnvalue_4 _returnvalue_3)
          (`EnhancedInputSubsystemInterface.AddMappingContext` (pcsubsystem `EnhancedInputLocalPlayerSubsystem` _returnvalue_4) "/Game/Pong/Input/IMC_Keyboard.IMC_Keyboard" 0 (struct))))
      (:`then_1`
        ;[1 1 1] Set initial camera position and save Ball Actor variables
        (bind _returnvalue_5 (`GameplayStatics.GetActorOfClass` "/Game/Pong/Blueprints/BP_CameraActor.BP_CameraActor_C"))
        (`PlayerController.SetViewTargetWithBlend` _returnvalue _returnvalue_5 0.0 "VTBlend_Linear" 0.0 false)
        (bind _returnvalue_6 (`GameplayStatics.GetActorOfClass` "/Game/Pong/Blueprints/BP_BallPawn.BP_BallPawn_C"))
        (bind _output_get (set `self.ball_actor` _returnvalue_6))
        (`/Game/Pong/Blueprints/BP_BallPawn.ChangeShape` _output_get))
      (:`then_2`
        ;[1 1 1] Adds Scoreboard to Viewport, save Game Instance
        (bind _returnvalue_7 (`|CreateWidget` "/Game/Pong/UI/WBP_Scoreboard.WBP_Scoreboard_C" _returnvalue))
        (`UserWidget.AddToViewport` _returnvalue_7 0)
        (bind _aspong_game_instance (cast `/Game/Pong/Blueprints/Pong_GameInstance` (`GameplayStatics.GetGameInstance`)))
        (set `self.gameinstance` _aspong_game_instance)))))

(event `ResetBallEvent`
  (bind _ball_actor (`self.ball_actor`))
  ;[1 1 1] Reset Ball Location if Score is Not >= MaxScore
  (set `/Game/Pong/Blueprints/BP_BallPawn.bReset` true _ball_actor)
  (`/Game/Pong/Blueprints/BP_BallPawn.ResetBallLocation` _ball_actor)
  (`/Game/Pong/Blueprints/BP_BallPawn.IncreaseBallVelocity` _ball_actor)
  (`KismetSystemLibrary.Delay` 1.5)
  (`/Game/Pong/Blueprints/BP_BallPawn.ResetBallVelocity` _ball_actor)
  (set `/Game/Pong/Blueprints/BP_BallPawn.bReset` false _ball_actor))

(event `GameOver`
  ;[1 1 1] Activate Game Over screen
  (bind _returnvalue (`|CreateWidget` "/Game/Pong/UI/WBP_GameOver.WBP_GameOver_C"))
  (`UserWidget.AddToViewport` _returnvalue 0)
  (set `PlayerController.bShowMouseCursor` true (`GameplayStatics.GetPlayerController` 0))
  (`GameplayStatics.SetGamePaused` true))

(fn `AddScoreP1`
  ;[1 1 1] Sets Score Values for Total
  (set `self.ScoreP1` (+ (`self.ScoreP1`) 1))
  (set `/Game/Pong/Blueprints/BP_BallPawn.bWinSide` true (`self.ball_actor`)))

(fn `AddScoreP2`
  ;[1 1 1] Sets Score Values for Total
  (set `self.ScoreP2` (+ (`self.ScoreP2`) 1))
  (set `/Game/Pong/Blueprints/BP_BallPawn.bWinSide` false (`self.ball_actor`)))

(fn `TrackScore`
  (bind _maxscore (`/Game/Pong/Blueprints/Pong_GameInstance.MaxScore` (`self.gameinstance`)))
  ;[1 1 1] Tracks When The Score Reaches MaxScore
  (if (>= (`self.ScoreP1`) _maxscore)
    (`self.GameOver` :!label _label)
    (elif (>= (`self.ScoreP2`) _maxscore)
      (goto _label)
      (else
        (`self.ResetBallEvent`)))))

(fn `UserConstructionScript`)